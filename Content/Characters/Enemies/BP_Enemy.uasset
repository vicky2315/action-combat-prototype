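; BP_Enemy is an enemy character that runs the BT_Enemy behavior tree through its AI controller when play begins.
; It links its world health bar widget to itself, hides it after a short delay, then binds a damage delegate that briefly shows it again for the passed duration.
; OnSelect and DeSelect events toggle a lock-on widget to mark the enemy as targeted.
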(event Custom|OnReceivedDamageDelegate_Event
  (params (Duration :type Float%20%28single-precision%29))
  (Rendering|SetVisibility (Variables|Default|GetHealthBarWidget) true false)
  (Utilities|FlowControl|Delay Duration)
  (Rendering|SetVisibility (Variables|Default|GetHealthBarWidget) false false))

(event EventOnSelect
  (Rendering|SetVisibility (Variables|Default|GetLockOnWidget) true false))

(event EventDeSelect
  (Rendering|SetVisibility (Variables|Default|GetLockOnWidget) false false))

(event EventBeginPlay
  (AI|RunBehaviorTree (AI|GetAIController self) "/Game/Characters/AI/BT_Enemy.BT_Enemy")
  (bind _aswbp_health_bar (Utilities|Casting|CastToWBP_HealthBar (UserInterface|GetUserWidgetObject (Variables|Default|GetHealthBarWidget))))
  (Variables|/Game/UI/WidgetBlueprints/GameWidgets/WBP_HealthBar.WBP_HealthBar_C|SetEnemyCharacter _aswbp_health_bar self)
  (Utilities|FlowControl|Delay 3.0)
  (Rendering|SetVisibility (Variables|Default|GetHealthBarWidget) false false)
  (EventDispatchers|AssignOnReceivedDamageDelegate (delegate Custom|OnReceivedDamageDelegate_Event)))

(fn ConstructionScript)